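; Exhibit stand for a virtual fair (FeriaVirtual) that displays a project's artwork and passes its details to the player.
; On BeginPlay it applies per-instance materials to the model's two image slots, falling back to black, and to its infographic slot.
; ShowProjectInfo writes the title, author and a Spanish "press F" prompt to the FeriaVirtualCharacter and sets an interactable flag.
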(event EventBeginPlay
  (bind _standmodel (Variables|Default|GetStandModel))
  (bind _standmodel_2 (Variables|Default|GetStandModel))
  (Utilities|IsValid (Variables|StandInfo|Getimage1)
    (:Is%20Valid
      (Rendering|Material|SetMaterialbyName _standmodel "img1" (Variables|StandInfo|Getimage1)))
    (:Is%20Not%20Valid
      (Rendering|Material|SetMaterialbyName _standmodel "img1" "/Game/3DModels/Feria_Virtual_Modelos/Models/Materials/Black.Black")))
  (Utilities|IsValid (Variables|StandInfo|Getimage2)
    (:Is%20Valid
      (Rendering|Material|SetMaterialbyName _standmodel_2 "img2" (Variables|StandInfo|Getimage2)))
    (:Is%20Not%20Valid
      (Rendering|Material|SetMaterialbyName _standmodel_2 "img2" "/Game/3DModels/Feria_Virtual_Modelos/Models/Materials/Black.Black")))
  (Rendering|Material|SetMaterialbyName (Variables|Default|GetStandModel) "Infografico" (Variables|StandInfo|Getinfografico)))

(fn ConstructionScript)

(fn ShowProjectInfo
  ;[0 0.06667 1] Asigna los valores de la obra al jugador
  (bind _asferia_virtual_character (Utilities|Casting|CastToFeriaVirtualCharacter (Game|GetPlayerCharacter 0)))
  (Variables|/Game/Blueprints/Characters/FeriaVirtual/FeriaVirtualCharacter.FeriaVirtualCharacter_C|SetInteractionMessage _asferia_virtual_character (Utilities|String|Append "Presiona \"F\" para interactuar con: " (Variables|Default|GetTitle)))
  (Variables|Default|SetInteractable true)
  (Utilities|FlowControl|Sequence
    (:then_0
      (Variables|/Game/Blueprints/Characters/FeriaVirtual/FeriaVirtualCharacter.FeriaVirtualCharacter_C|SetAuthor _asferia_virtual_character (Variables|Default|GetAuthor)))
    (:then_1
      (Variables|/Game/Blueprints/Characters/FeriaVirtual/FeriaVirtualCharacter.FeriaVirtualCharacter_C|SetTitle _asferia_virtual_character (Variables|Default|GetTitle)))
    (:then_2
      (Variables|Default|SetImage (Variables|Default|GetImage)))))