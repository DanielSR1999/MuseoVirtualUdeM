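; Game instance for a multiplayer virtual fair (Feria Virtual) that manages its UI and online sessions.
; Events show or remove login, message, loading, options and connected-player widgets, mostly creating each once and reusing it.
; Project display spawns the current Stand's infographic or video widget and locks movement until dismissed.
; Joining tries every non-full session found, then flows into session creation, which opens the fair level as a listen server.
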(event Custom|ShowMainMenu
  (bind _returnvalue (Game|GetPlayerController 0))
  ;[1 1 1] ShowMainMenu and set UI Mode
  (Utilities|IsValid (Variables|Default|GetLoginUIFeria)
    (:Is%20Valid
      _)
    (:Is%20Not%20Valid
      (bind _returnvalue_2 (UserInterface|CreateWidget "/Game/UI/Feria_de_la_Innovacion/LoginUIFeriaInnovacion.LoginUIFeriaInnovacion_C" 0 0))
      (bind _output_get (Variables|Default|SetLoginUIFeria _returnvalue_2))))
  (Input|SetInputModeUIOnly _returnvalue 0 "DoNotLock")
  (UserInterface|Viewport|AddtoViewport _output_get 0)
  (Variables|/Script/Engine.PlayerController|SetbShowMouseCursor _returnvalue true))

(event Custom|ShowOptionsMenuFeria
  ;[1 1 1] Show Options Menu
  (Utilities|IsValid (Variables|Default|GetOptionsMenuFeria)
    (:Is%20Valid
      _)
    (:Is%20Not%20Valid
      (bind _returnvalue (UserInterface|CreateWidget "/Game/UI/Feria_de_la_Innovacion/OptionsMenuFeria.OptionsMenuFeria_C" (Game|GetPlayerController 0)))
      (bind _output_get (Variables|Default|SetOptionsMenuFeria _returnvalue))))
  (UserInterface|Viewport|AddtoViewport _output_get 0))

(event Custom|JoinSesssion
  (bind _returnvalue (Game|GetPlayerController 0))
  ;[1 1 1] JoinSession
  (CallFunction|ShowLoadingScreenFeria)
  (bind _results (|FindSessions _returnvalue 20 false)
    (:OnSuccess
      (for _array_element _results
        (if (!= (Class|FindSessionsCallbackProxy|GetCurrentPlayers _array_element) (Class|FindSessionsCallbackProxy|GetMaxPlayers _array_element))
          (|JoinSession _returnvalue _array_element)))
      ;[1 1 1] Create session
      (|Session (Game|GetPlayerController 0) 50 false
        (:OnSuccess
          (Game|OpenLevel(byName) "FeriaVirtualGame" true "listen"))))))

(event Custom|ShowPlayersConnected
  ;[1 1 1] Show Players connected
  (Utilities|IsValid (Variables|Default|GetConnectedPlayersFeria)
    (:Is%20Not%20Valid
      (bind _returnvalue (UserInterface|CreateWidget "/Game/UI/Feria_de_la_Innovacion/ConnectedPlayersUIFeria.ConnectedPlayersUIFeria_C" (Game|GetPlayerController 0)))
      (bind _output_get (Variables|Default|SetConnectedPlayersFeria _returnvalue))
      (UserInterface|Viewport|AddtoViewport _output_get 0))))

(event Custom|CreateSession
  ;[1 1 1] Create session
  (CallFunction|ShowLoadingScreenFeria)
  (|Session (Game|GetPlayerController 0) 50 false
    (:OnSuccess
      (Game|OpenLevel(byName) "FeriaVirtualGame" true "listen"))))

(event Custom|ShowLoadingScreenFeria
  ;[1 1 1] Show Loading Screen
  (Utilities|IsValid (Variables|Default|GetLoadingScreenFeria)
    (:Is%20Valid
      _)
    (:Is%20Not%20Valid
      (bind _returnvalue (UserInterface|CreateWidget "/Game/UI/Feria_de_la_Innovacion/LoadingScreenUIFeria.LoadingScreenUIFeria_C" (Game|GetPlayerController 0)))
      (bind _output_get (Variables|Default|SetLoadingScreenFeria _returnvalue))))
  (UserInterface|Viewport|AddtoViewport _output_get 0))

(event Custom|DisableLogin
  ;[1 1 1] Disable Login
  (Utilities|IsValid (Variables|Default|GetLoginUIFeria)
    (:Is%20Valid
      (Widget|RemovefromParent (Variables|Default|GetLoginUIFeria)))))

(event Custom|ShowInteractionMessage
  ;[1 1 1] ShowArtWorkMessages
  (Utilities|IsValid (Variables|Default|GetMessagesScreenFeria)
    (:Is%20Valid
      _)
    (:Is%20Not%20Valid
      (bind _returnvalue (UserInterface|CreateWidget "/Game/UI/Feria_de_la_Innovacion/MessageScreenFeria.MessageScreenFeria_C" (Game|GetPlayerController 0)))
      (bind _output_get (Variables|Default|SetMessagesScreenFeria _returnvalue))))
  (UserInterface|Viewport|AddtoViewport _output_get 0))

(event Custom|ShowProjectWidget
  (bind _returnvalue (Game|GetPlayerController 0))
  ;[1 1 1] Show ArtWork Widget
  (bind _asferia_virtual_character (Utilities|Casting|CastToFeriaVirtualCharacter (Game|GetPlayerCharacter 0)))
  (Variables|Default|SetCharacterFeriaVirtual _asferia_virtual_character)
  (bind _asstand (Utilities|Casting|CastToStand (Variables|/Game/Blueprints/Characters/FeriaVirtual/FeriaVirtualCharacter.FeriaVirtualCharacter_C|GetCurrentInteractable _asferia_virtual_character)))
  (if (Variables|/Game/Blueprints/FeriaVirtual/Stand.Stand_C|GetInteractableInfografico _asstand)
    (bind _artworkwidget (Default|EnableInfograficoWidget _asstand))
    (bind _returnvalue_2 (UserInterface|CreateWidget _artworkwidget))
    (bind _output_get (Variables|Default|SetInfograficoWidget _returnvalue_2))
    (UserInterface|Viewport|AddtoViewport _output_get 0)
    (Input|SetInputModeUIOnly _returnvalue 0 "DoNotLock" :!label _label)
    (Variables|/Script/Engine.PlayerController|SetbShowMouseCursor _returnvalue true)
    (Pawn|Components|CharacterMovement|DisableMovement (Variables|/Script/Engine.Character|GetCharacterMovement (Variables|Default|GetCharacterFeriaVirtual)))
    (Variables|/Game/Blueprints/Characters/FeriaVirtual/FeriaVirtualCharacter.FeriaVirtualCharacter_C|SetInGameplay (Variables|Default|GetCharacterFeriaVirtual) false)
    (Variables|/Game/Blueprints/Characters/FeriaVirtual/FeriaVirtualCharacter.FeriaVirtualCharacter_C|SetUIEnabled (Variables|Default|GetCharacterFeriaVirtual) true)
    (elif (Variables|/Game/Blueprints/FeriaVirtual/Stand.Stand_C|GetInteractableVideo _asstand)
      (bind _artworkwidget_2 (Default|EnableSpotWidget _asstand))
      (bind _returnvalue_3 (UserInterface|CreateWidget _artworkwidget_2))
      (bind _output_get_2 (Variables|Default|SetSpotWidget _returnvalue_3))
      (UserInterface|Viewport|AddtoViewport _output_get_2 0)
      (goto _label))))

(event Custom|DisableProjectWidget
  (params (Widget :type User%20Widget%20Object%20Reference))
  (bind _characterferiavirtual (Variables|Default|GetCharacterFeriaVirtual))
  (bind _characterferiavirtual_2 (Variables|Default|GetCharacterFeriaVirtual))
  ;[1 1 1] DisableArtWorkWidget
  (if (Variables|/Game/Blueprints/Characters/FeriaVirtual/FeriaVirtualCharacter.FeriaVirtualCharacter_C|GetUIEnabled _characterferiavirtual_2)
    (Default|EnablePlayerMovement _characterferiavirtual_2)
    (Variables|/Game/Blueprints/Characters/FeriaVirtual/FeriaVirtualCharacter.FeriaVirtualCharacter_C|SetInGameplay _characterferiavirtual true)
    (Variables|/Game/Blueprints/Characters/FeriaVirtual/FeriaVirtualCharacter.FeriaVirtualCharacter_C|SetUIEnabled _characterferiavirtual false)
    (Widget|RemovefromParent Widget)))

(event Custom|DisableMessageScreen
  (bind _messagesscreenferia (Variables|Default|GetMessagesScreenFeria))
  ;[1 1 1] Disable Message Screen
  (Utilities|IsValid _messagesscreenferia
    (:Is%20Valid
      (Widget|RemovefromParent _messagesscreenferia))))